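; Base gamemode Blueprint that starts either the singleplayer first-person mode or the main menu.
; BeginPlay caches the GameInstance and player, loads settings, then picks singleplayer for "Playground" levels, otherwise following GamemodeMenu, which GamemodeUpdated_Event_0 rechecks.
; Main menu adds its widget, audio and saved Music/SFX volumes; singleplayer adds audio and calls CameraViewGame, currently an empty stub.
; CameraViewMenu sets cursor, UI-only input and disabled movement, but is uncalled here.
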(event `self.ReceiveBeginPlay`
  ;[0 0.09896 0.03931] Gamemode Base for all modes (current total 2)
  (`|ExecutionSequence`
    (:`then_0`
      (bind _setlocalvariableforgi (`/Game/Structure/BFL_CommonFunctions.SetupGameInstance`))
      (set `self.GameInstance` _setlocalvariableforgi)
      (bind _set_local_variable_for_player (`/Game/Structure/BFL_CommonFunctions.SetupFirstPersonCharacter`))
      (set `self.Player` _set_local_variable_for_player))
    (:`then_1`
      (`/Game/Structure/BP_GameInstance.GetPlayerGameSettings` (`self.GameInstance`)))
    (:`then_2`
      (bind _returnvalue (`GameplayStatics.GetCurrentLevelName` true))
      (if (`KismetStringLibrary.StartsWith` _returnvalue "Playground")
        (`self.Activate Singleplayer` :!label _label)
        (else
          (if (`/Game/Structure/BP_GameInstance.GamemodeMenu` (`self.GameInstance`)) :!label _label_2
            (`self.Activate Mainmenu`)
            (else
              (goto _label))))))))

(event `GamemodeUpdated_Event_0`
  ;[0 0.09896 0.03931] Gamemode Base for all modes (current total 2)
  (add `/Game/Structure/BP_GameInstance.GamemodeUpdated` (`self.GameInstance`) (delegate `GamemodeUpdated_Event_0`))
  (goto _label_2))

(event `Activate Singleplayer`
  ;[0 0.09896 0.03931] Gamemode Singleplayer & first person
  (`|ExecutionSequence`
    (:`then_0`
      (`self.CameraView_Game`))
    (:`then_1`
      (`AddComponent|NODE_AddAudioComponent-4`))))

(event `Activate Mainmenu`
  ;[0 0.09896 0.03931] Gamemode Mainmenu
  (`|ExecutionSequence`
    (:`then_0`
      (bind _returnvalue (`|CreateWidget` "/Game/Structure/Widgets/WB_MainMenu.WB_MainMenu_C"))
      (`UserWidget.AddToViewport` _returnvalue 0))
    (:`then_1`
      (`AddComponent|NODE_AddAudioComponent-5`)
      (`GameplayStatics.SetSoundMixClassOverride` "/Game/Resources/Audio/SoundMixModifier/MainSoundMix.MainSoundMix" "/Game/Resources/Audio/SoundClass/SC_Music.SC_Music" (`/Game/Structure/BP_SaveSettings.VolumeMusic` (`/Game/Structure/BP_GameInstance.PlayerSettings` (`self.GameInstance`))) 1.0 0.0)
      (`GameplayStatics.PushSoundMixModifier` "/Game/Resources/Audio/SoundMixModifier/MainSoundMix.MainSoundMix"))
    (:`then_2`
      (`GameplayStatics.SetSoundMixClassOverride` "/Game/Resources/Audio/SoundMixModifier/MainSoundMix.MainSoundMix" "/Game/Resources/Audio/SoundClass/SC_SFX.SC_SFX" (`/Game/Structure/BP_SaveSettings.VolumeSFX` (`/Game/Structure/BP_GameInstance.PlayerSettings` (`self.GameInstance`))) 1.0 0.0)
      (`GameplayStatics.PushSoundMixModifier` "/Game/Resources/Audio/SoundMixModifier/MainSoundMix.MainSoundMix"))))

(fn `CameraView_Game`)

(fn `CameraView_Menu`
  (bind _player (`self.Player`))
  (`|ExecutionSequence`
    (:`then_0`
      (`ActorComponent.Activate` (`Actor.RootComponent` _player) false)
      (`PlayerController.SetViewTargetWithBlend` (`GameplayStatics.GetPlayerController` 0) (`ActorComponent.GetOwner` (`Actor.RootComponent` _player)) 0.0 "VTBlend_Linear" 0.0 false)
      (set `PlayerCameraManager.bUseCameraHeightAsViewTarget` true (`PlayerController.PlayerCameraManager` (`GameplayStatics.GetPlayerController` 0))))
    (:`then_1`
      (bind _asplayer_controller (cast `PlayerController` (`Pawn.GetController` (`GameplayStatics.GetPlayerPawn` 0))))
      (set `PlayerController.bShowMouseCursor` true _asplayer_controller)
      (`WidgetBlueprintLibrary.SetInputMode_UIOnlyEx` (`GameplayStatics.GetPlayerController` 0) null))
    (:`then_2`
      (bind _set_local_variable_for_player (`/Game/Structure/BFL_CommonFunctions.SetupFirstPersonCharacter`))
      (`CharacterMovementComponent.DisableMovement` (`Character.CharacterMovement` _set_local_variable_for_player)))))

(fn `UserConstructionScript`)